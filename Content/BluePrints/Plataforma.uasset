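; Plataforma is a moving platform actor that slides between two offsets from its starting location.
; BeginPlay stores the initial position and plays the Plataforma timeline from the start.
; Each timeline update uses the Platf track as the alpha to lerp between PosA and PosB added to that position, setting the location without sweep.
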(event `self.ReceiveBeginPlay`
  (set `self.PosInicial` (`self.K2_GetActorLocation`))
  (bind (_direction _platf) (`Timeline|Plataforma` :!via `PlayFromStart`)
    (:`Update`
      (`self.K2_SetActorLocation` (`KismetMathLibrary.VLerp` (+ (`self.PosInicial`) (`self.PosA`)) (+ (`self.PosB`) (`self.PosInicial`)) _platf)))))

(fn `UserConstructionScript`)