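; Melee enemy character that spots the living player through PawnSensing, chases with AI MoveTo and punches on arrival.
; Combat plays the attack montage and sound, with a delayed reset; punch collider overlaps damage the player while punching, with collision toggled by separate events.
; TakeDamage disables that collider, then plays a hit montage or, at zero health, flags death, disables capsule collision and stops montages.
; An experimental, locally uncalled event flips facing along X.
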(event `self.PawnSensing.OnSeePawn`
  (params (Pawn :type "Pawn Object Reference"))
  ; DETECTAR PLAYER
  (if (and (not (`self.Death`)) (not (`self.Is Punching`)))
    (bind _asprota (cast `/Game/BluePrints/Prota` Pawn))
    (if (not (`/Game/BluePrints/Prota.Muerto` _asprota))
      (`self.Follow` _asprota))))

(event `Follow`
  (params (Player :type "Actor Object Reference"))
  ; FOLLOW
  (`|AIMoveTo` self (0.0 0.0 0.0) Player 100.0
    (:`OnSuccess`
      (`self.Combat`))))

(event `Combat`
  ; ATTACK
  (if (not (and (`self.Attack`) (`self.Is Punching`)))
    (bind _returnvalue (`self.PlayAnimMontage` "/Game/Characters/Enemy1/Anims/AttackMontage.AttackMontage"))
    (set `self.Attack` true)
    (set `self.Is Punching` true)
    (`GameplayStatics.PlaySoundAtLocation` "/Game/Audio/Attack/PunchEnemy.PunchEnemy" (`self.K2_GetActorLocation`) (struct) 0.6 1.0 0.01 null null null null)
    (`KismetSystemLibrary.Delay` _returnvalue)
    (`KismetSystemLibrary.Delay` 1.0)
    (set `self.Is Punching` false)
    (set `self.Attack` false)))

(event `TakeDamage`
  (params (Damage :type "Float (double-precision)"))
  ; ATTACK
  (`self.DesactivatePunchCollider`)
  (bind _output_get (set `self.Health` (- (`self.Health`) Damage)))
  (if (<= _output_get 0.0)
    (set `self.Death` true)
    (`PrimitiveComponent.SetCollisionEnabled` (`self.CapsuleComponent`) "NoCollision")
    (`self.StopAnimMontage` "/Game/Characters/Enemy1/Anims/HitMontage.HitMontage")
    (`self.StopAnimMontage` "/Game/Characters/Enemy1/Anims/AttackMontage.AttackMontage")
    (`GameplayStatics.PlaySoundAtLocation` "/Game/Audio/EnemyHurt.EnemyHurt" (`self.K2_GetActorLocation`) (struct) 0.8 1.0 0.0 null null null null)
    (else
      (`self.PlayAnimMontage` "/Game/Characters/Enemy1/Anims/HitMontage.HitMontage"))))

(event `self.PunchColider.OnComponentBeginOverlap`
  (params (OverlappedComponent :type "PrimitiveComponent Object Reference") (OtherActor :type "Actor Object Reference") (OtherComp :type "PrimitiveComponent Object Reference") (OtherBodyIndex :type Integer) (bFromSweep :type Boolean) (SweepResult :type "HitResult Structure (by ref)"))
  ; ATTACK
  (bind _asprota (cast `/Game/BluePrints/Prota` OtherActor))
  (if (`self.Is Punching`)
    (`/Game/BluePrints/Prota.TakeDamage` _asprota (`self.Damage`) false)))

(event `ActivatePunchCollider`
  ; PUNCH COLLIDER
  (`PrimitiveComponent.SetCollisionEnabled` (`self.PunchColider`) "QueryOnly"))

(event `MirarPlayer`
  (params (Player :type "Actor Object Reference"))
  (bind _returnvalue_x (`KismetMathLibrary.BreakVector` (`self.K2_GetActorLocation` Player)))
  (bind _returnvalue_x_2 (`KismetMathLibrary.BreakVector` (`self.K2_GetActorLocation`)))
  ; CAMBIAR ROTACION ENEMIGO (PRUEBA)
  (if (> _returnvalue_x _returnvalue_x_2)
    (`self.K2_SetActorRotation` (struct))
    (else
      (`self.K2_SetActorRotation` (`KismetMathLibrary.MakeRotator` 0.0 0.0 180.0)))))

(event `DesactivatePunchCollider`
  ; PUNCH COLLIDER
  (`PrimitiveComponent.SetCollisionEnabled` (`self.PunchColider`) "NoCollision"))

(fn `UserConstructionScript`)