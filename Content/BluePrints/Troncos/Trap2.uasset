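; Trap2 is a log trap that moves and rotates, damaging and knocking back the Prota player character on overlap.
; From BeginPlay, one timeline lerps it between two offsets from its start position, and its updates play a second timeline driving yaw.
; An overlap with a living Prota deals damage and disables input.
; A self-calling delayed event then pushes the player along world +X in growing steps, restoring input afterwards if still alive.
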(event `self.ReceiveActorBeginOverlap`
  (params (OtherActor :type "Actor Object Reference"))
  (bind _asprota (cast `/Game/BluePrints/Prota` OtherActor))
  (if (not (`/Game/BluePrints/Prota.Muerto` _asprota))
    (`/Game/BluePrints/Prota.TakeDamage` _asprota 20.0 false)
    (set `self.As Prota` _asprota)
    (`self.DisableInput` _asprota (`GameplayStatics.GetPlayerController` 0))
    (set `self.Alpha` 0.0)
    (`self.DesplazarPlayer`)))

(event `DesplazarPlayer`
  (bind _alpha (`self.Alpha`))
  (bind _as_prota (`self.As Prota`))
  (bind _as_prota_2 (`self.As Prota`))
  (bind (_returnvalue_x _returnvalue_y _returnvalue_z) (`KismetMathLibrary.BreakVector` (`self.K2_GetActorLocation` _as_prota_2)))
  (set `self.Alpha` (+ (`self.Alpha`) 0.2))
  (`self.K2_SetActorLocation` _as_prota (`KismetMathLibrary.VLerp` (`self.K2_GetActorLocation` _as_prota_2) (`KismetMathLibrary.MakeVector` (+ _returnvalue_x 50.0) _returnvalue_y _returnvalue_z) _alpha) false false)
  (`KismetSystemLibrary.Delay` 0.02)
  (if (< _alpha 1.0)
    (`self.DesplazarPlayer`)
    (elif (not (`/Game/BluePrints/Prota.Muerto` _as_prota))
      (`self.EnableInput` _as_prota (`GameplayStatics.GetPlayerController` 0)))))

(event `self.ReceiveBeginPlay`
  (bind (_returnvalue_roll _returnvalue_pitch) (`KismetMathLibrary.BreakRotator` (`self.K2_GetActorRotation`)))
  (set `self.PosInicial` (`self.K2_GetActorLocation`))
  (bind (_direction _tronco) (`Timeline|MovimientoTronco` :!via `PlayFromStart`)
    (:`Update`
      (`self.K2_SetActorLocation` (`KismetMathLibrary.VLerp` (+ (`self.PosInicial`) (`self.PosA`)) (+ (`self.PosB`) (`self.PosInicial`)) _tronco))
      (bind (_direction_2 _newtrack_0) (`Timeline|RotationTronco`)
        (:`Update`
          (`self.K2_SetActorRotation` (`KismetMathLibrary.MakeRotator` _returnvalue_roll _returnvalue_pitch _newtrack_0)))))))

(fn `UserConstructionScript`)