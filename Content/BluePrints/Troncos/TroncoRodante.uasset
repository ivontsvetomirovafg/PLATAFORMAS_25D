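; TroncoRodante is a rolling-log hazard that damages and knocks back the Prota character when it overlaps the log's capsule.
; On overlap it applies damage, disables player input and starts Empujar, a self-calling event paced by a short Delay.
; Each step lerps from the player's current location toward a +Y world offset with rising Alpha, so the push accumulates without sweeping.
; When Alpha completes, input returns and the log destroys itself.
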(event `self.Capsule.OnComponentBeginOverlap`
  (params (OverlappedComponent :type "PrimitiveComponent Object Reference") (OtherActor :type "Actor Object Reference") (OtherComp :type "PrimitiveComponent Object Reference") (OtherBodyIndex :type Integer) (bFromSweep :type Boolean) (SweepResult :type "HitResult Structure (by ref)"))
  (bind _asprota (cast `/Game/BluePrints/Prota` OtherActor))
  (`/Game/BluePrints/Prota.TakeDamage` _asprota 20.0 false)
  (set `self.As Prota` _asprota)
  (`self.DisableInput` _asprota (`GameplayStatics.GetPlayerController` 0))
  (set `self.Alpha` 0.0)
  (`self.Empujar`))

(event `Empujar`
  (bind _alpha (`self.Alpha`))
  (bind _as_prota (`self.As Prota`))
  (bind _as_prota_2 (`self.As Prota`))
  (bind (_returnvalue_x _returnvalue_y _returnvalue_z) (`KismetMathLibrary.BreakVector` (`self.K2_GetActorLocation` _as_prota_2)))
  (set `self.Alpha` (+ (`self.Alpha`) 0.2))
  (`self.K2_SetActorLocation` _as_prota (`KismetMathLibrary.VLerp` (`self.K2_GetActorLocation` _as_prota_2) (`KismetMathLibrary.MakeVector` _returnvalue_x (+ _returnvalue_y 50.0) _returnvalue_z) _alpha) false false)
  (`KismetSystemLibrary.Delay` 0.02)
  (if (< _alpha 1.0)
    (`self.Empujar`)
    (else
      (`self.EnableInput` _as_prota (`GameplayStatics.GetPlayerController` 0))
      (`self.K2_DestroyActor`))))

(fn `UserConstructionScript`)