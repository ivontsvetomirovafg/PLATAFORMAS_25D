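; GiroEsquina is a corner-turn trigger that changes the path direction of the Prota player character when it overlaps.
; On overlap it toggles the player's AnguloCamino between AnguloAntes and NuevoAngulo, so the corner works in both directions of travel.
; It then moves the player to the trigger's world location to re-center them on the turn.
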(event `self.Trigger.OnComponentBeginOverlap`
  (params (OverlappedComponent :type "PrimitiveComponent Object Reference") (OtherActor :type "Actor Object Reference") (OtherComp :type "PrimitiveComponent Object Reference") (OtherBodyIndex :type Integer) (bFromSweep :type Boolean) (SweepResult :type "HitResult Structure (by ref)"))
  ; Cambiar dirección Player
  (bind _asprota (cast `/Game/BluePrints/Prota` OtherActor))
  (if (== (`/Game/BluePrints/Prota.AnguloCamino` _asprota) (`self.AnguloAntes`))
    (set `/Game/BluePrints/Prota.AnguloCamino` (`self.NuevoAngulo`) _asprota)
    (else
      (set `/Game/BluePrints/Prota.AnguloCamino` (`self.AnguloAntes`) _asprota)))
  (`self.K2_SetActorLocation` _asprota (`KismetMathLibrary.MakeVector` (.x (`SceneComponent.K2_GetComponentLocation` (`self.Trigger`))) (.y (`SceneComponent.K2_GetComponentLocation` (`self.Trigger`))) (.z (`SceneComponent.K2_GetComponentLocation` (`self.Trigger`)))) false false))

(fn `UserConstructionScript`)