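; Trap Blueprint that damages the Prota character on overlap and drags it 300 units along world X from the trap's location.
; On overlap it applies damage and disables player input, then re-enables input once the move completes.
; The move is a stepped lerp in a while loop with a Delay between small alpha increments, setting location without sweep.
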(event `self.ReceiveActorBeginOverlap`
  (params (OtherActor :type "Actor Object Reference"))
  (bind (_returnvalue_x _returnvalue_y _returnvalue_z) (`KismetMathLibrary.BreakVector` (`self.K2_GetActorLocation`)))
  (bind _alpha (`self.Alpha`))
  (bind _asprota (cast `/Game/BluePrints/Prota` OtherActor))
  (`/Game/BluePrints/Prota.TakeDamage` _asprota 20.0)
  (`self.DisableInput` _asprota (`GameplayStatics.GetPlayerController` 0))
  (set `self.Alpha` 0.0)
  (while (< _alpha 1.0)
    (set `self.Alpha` (+ (`self.Alpha`) 0.01))
    (`self.K2_SetActorLocation` _asprota (`KismetMathLibrary.VLerp` (`self.K2_GetActorLocation`) (`KismetMathLibrary.MakeVector` (+ _returnvalue_x 300.0) _returnvalue_y _returnvalue_z) _alpha) false false)
    (`KismetSystemLibrary.Delay` 0.5))
  (`self.EnableInput` _asprota (`GameplayStatics.GetPlayerController` 0)))

(fn `UserConstructionScript`)