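; Enemy2 is an enemy character that chases the Prota player and attacks from range.
; Pawn sensing triggers an AI move toward the living player, and reaching the acceptance radius starts the attack.
; The attack plays a montage and sound, then spawns a SpawnAttack actor at the Sphere with the enemy's level-two flag, gated by delays.
; Damage plays a hit montage or, at zero health, flags death and disables capsule collision.
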(event `self.PawnSensing.OnSeePawn`
  (params (Pawn :type "Pawn Object Reference"))
  ; DETECTAR PLAYER
  (if (not (`self.Death`))
    (bind _asprota (cast `/Game/BluePrints/Prota` Pawn))
    (if (not (`/Game/BluePrints/Prota.Muerto` _asprota))
      (`self.Follow` _asprota))))

(event `MirarPlayer`
  (params (Player :type "Actor Object Reference"))
  (bind _returnvalue_x (`KismetMathLibrary.BreakVector` (`self.K2_GetActorLocation` Player)))
  (bind _returnvalue_x_2 (`KismetMathLibrary.BreakVector` (`self.K2_GetActorLocation`)))
  ; CAMBIAR ROTACION ENEMIGO (PRUEBA)
  (if (> _returnvalue_x _returnvalue_x_2)
    (`self.K2_SetActorRotation` (struct))
    (else
      (`self.K2_SetActorRotation` (`KismetMathLibrary.MakeRotator` 0.0 0.0 270.0)))))

(event `Follow`
  (params (Player :type "Actor Object Reference"))
  ; FOLLOW
  (`|AIMoveTo` self (0.0 0.0 0.0) Player 600.0
    (:`OnSuccess`
      (`self.Attack `))))

(event `Attack`
  (bind _sphere (`self.Sphere`))
  ; ATTACK
  (if (not (`self.Attack`))
    (`self.PlayAnimMontage` "/Game/Characters/Enemy2/Anims/Attack.Attack")
    (set `self.Attack` true)
    (`GameplayStatics.PlaySoundAtLocation` "/Game/Audio/Attack/AttackEnemy2.AttackEnemy2" (`self.K2_GetActorLocation`) (struct) 0.6 1.0 0.0 null null null null)
    (`KismetSystemLibrary.Delay` 1.0)
    (bind _returnvalue (`|SpawnActorFromClass` "/Game/BluePrints/SpawnAttack.SpawnAttack_C" (`KismetMathLibrary.MakeTransform` (`SceneComponent.K2_GetComponentLocation` _sphere) (`SceneComponent.K2_GetComponentRotation` _sphere)) "Undefined" "MultiplyWithRoot" null null))
    (set `/Game/BluePrints/SpawnAttack.Lvl2` (`self.Lvl2Enemy`) _returnvalue)
    (`KismetSystemLibrary.Delay` 1.5)
    (set `self.Attack` false)))

(event `TakeDamage`
  (params (Damage :type "Float (double-precision)"))
  ; ATTACK
  (bind _output_get (set `self.Health` (- (`self.Health`) Damage)))
  (if (<= _output_get 0.0)
    (set `self.Death` true)
    (`PrimitiveComponent.SetCollisionEnabled` (`self.CapsuleComponent`) "NoCollision")
    (`self.StopAnimMontage` "/Game/Characters/Enemy2/Anims/Hit.Hit")
    (`self.StopAnimMontage` "/Game/Characters/Enemy2/Anims/Attack.Attack")
    (`GameplayStatics.PlaySoundAtLocation` "/Game/Audio/EnemyHurt2.EnemyHurt2" (`self.K2_GetActorLocation`) (struct) 0.8 1.0 0.01 null null null null)
    (else
      (`self.PlayAnimMontage` "/Game/Characters/Enemy2/Anims/Hit.Hit"))))

(fn `UserConstructionScript`)