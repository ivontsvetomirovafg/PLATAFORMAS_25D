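; SpawnAttack is a moving hazard actor that damages the Prota player character on contact.
; Each tick it moves in a straight line, along +X by default or along -Y when Lvl2 is set, scaled by Speed and delta time.
; On overlap with Prota, the Coll component applies non-water damage, disables its collision and destroys the actor.
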(event `self.ReceiveTick`
  (params (DeltaSeconds :type "Float (single-precision)"))
  (bind (_returnvalue_x _returnvalue_y _returnvalue_z) (`KismetMathLibrary.BreakVector` (`self.K2_GetActorLocation`)))
  (bind (_returnvalue_x_2 _returnvalue_y_2 _returnvalue_z_2) (`KismetMathLibrary.BreakVector` (`self.K2_GetActorLocation`)))
  (if (`self.Lvl2`)
    (`self.K2_SetActorLocation` (`KismetMathLibrary.MakeVector` _returnvalue_x_2 (+ _returnvalue_y_2 (* (* (`self.Speed`) -1.0) DeltaSeconds)) _returnvalue_z_2))
    (else
      (`self.K2_SetActorLocation` (`KismetMathLibrary.MakeVector` (+ _returnvalue_x (* (`self.Speed`) DeltaSeconds)) _returnvalue_y _returnvalue_z)))))

(event `self.Coll.OnComponentBeginOverlap`
  (params (OverlappedComponent :type "PrimitiveComponent Object Reference") (OtherActor :type "Actor Object Reference") (OtherComp :type "PrimitiveComponent Object Reference") (OtherBodyIndex :type Integer) (bFromSweep :type Boolean) (SweepResult :type "HitResult Structure (by ref)"))
  (bind _asprota (cast `/Game/BluePrints/Prota` OtherActor))
  (if true
    (`/Game/BluePrints/Prota.TakeDamage` _asprota (`self.Damage`) false)
    (`PrimitiveComponent.SetCollisionEnabled` (`self.Coll`) "NoCollision")
    (`self.K2_DestroyActor`)))

(fn `UserConstructionScript`)